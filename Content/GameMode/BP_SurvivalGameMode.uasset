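; Survival game mode Blueprint that presents the wave-based boss battle flow through music, wave messages and end screens.
; It binds to the survival state-change event and switches on each state, showing countdown or plain text widgets via two helper functions.
; The last wave also gets its own banner and spawn delay.
; Victory or death clears widgets, fades the camera to black, then async-loads the win or lose screen.
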(event `self.ReceiveBeginPlay`
  (`GameplayStatics.SpawnSound2D` "/Game/Assets/Sounds/Music/Dungeons_EndBossBattle.Dungeons_EndBossBattle" 1.0 1.0 0.0 null)
  (add `self.OnSurvivalGameModeChange` (delegate `OnSurvivalGameModeChange_Event`)))

(event `OnSurvivalGameModeChange_Event` :!signature `self.OnSurvivalGameModeChange`
  (params (CurrentState :type "EWarriorSurvivalGameModeState Enum" :default "WaitSpawnNewWave"))
  (switch `EWarriorSurvivalGameModeState` CurrentState
    (:`WaitSpawnNewWave`
      (`self.CreateWaveWidgetWithCountdown` (`|FormatText` "New Wave Coming In") (`self.SpawnNewWaveWaitTime`)))
    (:`SpawningNewWave`
      (`self.CreateWaveWidgetNoCountDown` (`|FormatText` "Wave {CurrentWaveCount}" (`self.CurrentWaveCount`)))
      (if (== (`self.CurrentWaveCount`) (`self.TotalWavesToSpawn`))
        (set `self.SpawnEnemiesDelayTime` 4.0)
        (`KismetSystemLibrary.Delay` 2.0)
        (`self.CreateWaveWidgetNoCountDown` "Last Wave")))
    (:`WaveCompleted`
      (`self.CreateWaveWidgetWithCountdown` (`|FormatText` "Wave {CurrentWaveCount} Completed" (`self.CurrentWaveCount`)) (`self.WaveCompletedWaitTime`)))
    (:`AllWavesDone`
      (`KismetSystemLibrary.Delay` 1.5)
      (`WidgetLayoutLibrary.RemoveAllWidgets`)
      (`PlayerCameraManager.StartCameraFade` :`self` (`GameplayStatics.GetPlayerCameraManager` 0) :`ToAlpha` 1.0 :`Duration` 3.0 :`bHoldWhenFinished` true)
      (`KismetSystemLibrary.Delay` 3.0)
      (bind _class (`|LoadAssetClass` "/Game/Widget/GameModeWidget/WBP_WinScreen.WBP_WinScreen_C")
        (:`Completed`
          (bind _asuser_widget (castclass `UserWidget` _class))
          (bind _returnvalue (`|CreateWidget` _asuser_widget))
          (`UserWidget.AddToViewport` _returnvalue 0))))
    (:`PlayerDied`
      (`WidgetLayoutLibrary.RemoveAllWidgets`)
      (`PlayerCameraManager.StartCameraFade` :`self` (`GameplayStatics.GetPlayerCameraManager` 0) :`ToAlpha` 1.0 :`Duration` 2.0 :`bHoldWhenFinished` true)
      (`KismetSystemLibrary.Delay` 2.0)
      (bind _class_2 (`|LoadAssetClass` "/Game/Widget/GameModeWidget/WBP_LooseScreen.WBP_LooseScreen_C")
        (:`Completed`
          (bind _asuser_widget_2 (castclass `UserWidget` _class_2))
          (bind _returnvalue_2 (`|CreateWidget` _asuser_widget_2))
          (`UserWidget.AddToViewport` _returnvalue_2 0))))))

(fn `CreateWaveWidgetNoCountDown`
  (params (TextContentToDisplay :type Text))
  (bind _returnvalue (`|CreateWidget` "/Game/Widget/GameModeWidget/WBP_WaveTextNoCountDown.WBP_WaveTextNoCountDown_C"))
  (`UserWidget.AddToViewport` _returnvalue 0)
  (set `TextBlock.Text` TextContentToDisplay (`/Game/Widget/GameModeWidget/WBP_WaveTextNoCountDown.TextBlock_WaveText` _returnvalue)))

(fn `CreateWaveWidgetWithCountdown`
  (params (TextContentToDisplay :type Text) (InTotalCountDownTime :type "Float (double-precision)"))
  (bind _returnvalue (`|GenericCreateObject` "/Game/Widget/GameModeWidget/WBP_WaitTextWithCountDown.WBP_WaitTextWithCountDown_C"))
  (`UserWidget.AddToViewport` _returnvalue 0)
  (set `TextBlock.Text` TextContentToDisplay (`/Game/Widget/GameModeWidget/WBP_WaitTextWithCountDown.TextBlock_WaveText` _returnvalue))
  (`/Game/Widget/GameModeWidget/WBP_WaitTextWithCountDown.StartCountDown` _returnvalue InTotalCountDownTime))

(fn `UserConstructionScript`)