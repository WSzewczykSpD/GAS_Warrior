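; Base projectile Blueprint that handles the sound and visual effects of a projectile's spawn and impact.
; BeginPlay plays a one-shot spawn sound and attaches a second sound to the root, stopped when the projectile is destroyed.
; OnSpawnProjectileHitEffects plays impact sound and FX at the hit location, and also spawns the muzzle FX at the projectile's current location, facing forward.
; Every asset is validity-checked, so each effect is optional.
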(event `self.ReceiveBeginPlay`
  (`|ExecutionSequence`
    (:`then_0`
      (bind _projectilespawnsound (`self.ProjectileSpawnSound`)
        (:`then`
          (`GameplayStatics.PlaySoundAtLocation` _projectilespawnsound (`self.K2_GetActorLocation`) (struct) 1.0 1.0 0.0 null null null null))
        (:`else`)))
    (:`then_1`
      (bind _projectileattachsound (`self.ProjectileAttachSound`)
        (:`then`
          (`GameplayStatics.SpawnSoundAttached` _projectileattachsound (`self.RootComponent`) "None" (0.0 0.0 0.0) (struct) "KeepRelativeOffset" true 1.0 1.0 0.0 null null))
        (:`else`)))))

(event `self.BP_OnSpawnProjectileHitEffects`
  (params (HitLocation :type "Vector Structure"))
  (`|ExecutionSequence`
    (:`then_0`
      (bind _projectile_impact_sound (`self.Projectile Impact Sound`)
        (:`then`
          (`GameplayStatics.PlaySoundAtLocation` _projectile_impact_sound HitLocation (struct) 1.0 1.0 0.0 null null null null))
        (:`else`)))
    (:`then_1`
      (bind _projectile_impact_fx (`self.Projectile Impact FX`)
        (:`then`
          (`NiagaraFunctionLibrary.SpawnSystemAtLocation` _projectile_impact_fx HitLocation))
        (:`else`)))
    (:`then_2`
      (bind _projectilemuzzlefx (`self.ProjectileMuzzleFX`)
        (:`then`
          (`NiagaraFunctionLibrary.SpawnSystemAtLocation` _projectilemuzzlefx (`self.K2_GetActorLocation`) (`KismetMathLibrary.Conv_VectorToRotator` (`self.GetActorForwardVector`))))
        (:`else`)))))

(fn `UserConstructionScript`)